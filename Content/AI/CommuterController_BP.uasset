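; AI controller Blueprint for a commuter character, which runs the BT_Commuter behavior tree on possess.
; StartEnemyTimer clears the HasLineOfSight and EnemyActor Blackboard keys.
; Disconnected logic would set those keys when a Player-tagged actor is sensed, or otherwise start a delayed timer to clear them.
; The perception update event is unwired, so this sight tracking never runs.
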(event `self.ReceivePossess`
  (params (PossessedPawn :type "Pawn Object Reference"))
  (`self.RunBehaviorTree` "/Game/AI/BT_Commuter.BT_Commuter"))

(event `self.AIPerception.OnTargetPerceptionUpdated`
  (params (Actor :type "Actor Object Reference") (Stimulus :type "AIStimulus Structure")))

(event `StartEnemyTimer`
  (bind _blackboard (`self.Blackboard`))
  (`BlackboardComponent.SetValueAsBool` _blackboard (`self.Has Line of Sight`) false)
  (`BlackboardComponent.SetValueAsObject` _blackboard (`self.Enemy Actor`) null))

(fn `UserConstructionScript`)