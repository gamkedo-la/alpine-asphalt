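; Spectator pawn that follows a wheeled vehicle from an elevated chase view at a fixed world-space offset.
; On BeginPlay it caches the first AA_WheeledVehiclePawn found in the level as the spectated target.
; Each Tick it moves behind and above that vehicle along world axes and sets the first player controller's rotation to look at it, without smoothing or validity checks.
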(event `self.ReceiveBeginPlay`
  (bind _outactors (`GameplayStatics.GetAllActorsOfClass` "/Script/AlpineAsphalt.AA_WheeledVehiclePawn"))
  (set `self.SpectatedVehicle` (`|GetArrayItem` _outactors)))

(event `self.ReceiveTick`
  (params (DeltaSeconds :type "Float (single-precision)"))
  (bind _returnvalue (`self.K2_GetActorLocation` (`self.SpectatedVehicle`)))
  (bind _returnvalue_2 (+ _returnvalue (-2500.0 0.0 2500.0)))
  (`self.K2_SetActorLocation` _returnvalue_2)
  (`Controller.SetControlRotation` (`GameplayStatics.GetPlayerController` 0) (`KismetMathLibrary.FindLookAtRotation` _returnvalue_2 _returnvalue)))

(fn `UserConstructionScript`)