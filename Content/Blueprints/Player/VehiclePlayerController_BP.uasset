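; Player controller for the driven vehicle that feeds speed and gear to the HUD and handles pause menu and map toggles.
; Each tick, FindSkidMax reads wheel contact, slip, skid and surface material to drive short force-feedback pulses: speed-scaled random rumble off-road, skid-scaled rumble on road.
; Pause pushes a menu through BaseUI and switches input mode.
; The map widget loads from a soft class and switches map capture on only while shown.
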(event `EnhancedInput|/Game/Input/Actions/IA_Toggle_Map`
  (params (ActionValue :type Boolean) (ElapsedSeconds :type "Float (double-precision)") (TriggeredSeconds :type "Float (double-precision)") (InputAction :type "InputAction Object Reference" :default "/Game/Input/Actions/IA_Toggle_Map.IA_Toggle_Map"))
  (:`Started`
    (`self.Toggle Map`)))

(event `EnhancedInput|/Game/Input/Actions/IA_Pause`
  (params (ActionValue :type Boolean) (ElapsedSeconds :type "Float (double-precision)") (TriggeredSeconds :type "Float (double-precision)") (InputAction :type "InputAction Object Reference" :default "/Game/Input/Actions/IA_Pause.IA_Pause"))
  (:`Completed`
    (`self.Run Pause`)))

(event `self.ReceiveBeginPlay`
  (bind _asvehicle_pawn_bp (cast `/Game/Blueprints/Vehicle/VehiclePawn_BP` (`self.K2_GetPawn`)))
  (set `self.Vehicle Movement Component` (`AA_WheeledVehiclePawn.VehicleMovementComponent` _asvehicle_pawn_bp)))

(event `self.ReceiveTick`
  (params (DeltaSeconds :type "Float (single-precision)"))
  (bind _vehicle_movement_component (`self.Vehicle Movement Component`))
  (`AA_VehicleUI.UpdateSpeed` (`self.VehicleUI`) (`ChaosVehicleMovementComponent.GetForwardSpeed` _vehicle_movement_component))
  (`AA_VehicleUI.UpdateGear` (`self.VehicleUI`) (`ChaosVehicleMovementComponent.GetCurrentGear` _vehicle_movement_component))
  (bind (_leftskid _rightskid _leftoffroad _rightoffroad) (`self.Find Skid Max`))
  (`|ExecutionSequence`
    (:`then_0`
      (if _leftoffroad
        ;[1 1 1] Offroad Rumble LEft
        (`self.PlayDynamicForceFeedback` (* (`KismetMathLibrary.RandomFloat`) (`KismetMathLibrary.MapRangeClamped` (`KismetMathLibrary.Abs` (`ChaosVehicleMovementComponent.GetForwardSpeedMPH` (`self.Vehicle Movement Component`))) 0.0 100.0 0.0 0.2)) 0.05 true false false false)
        (else
          ;[1 1 1] Left Wheel On Road Rumble
          (`self.PlayDynamicForceFeedback` (`KismetMathLibrary.MapRangeClamped` (/ (- _leftskid 500.0) 1000.0) 0.0 1.0 0.0 0.3) 0.05 false true false false))))
    (:`then_1`
      (if _rightoffroad
        ;[1 1 1] OffRoad Rumble Right
        (`self.PlayDynamicForceFeedback` (* (`KismetMathLibrary.RandomFloat`) (`KismetMathLibrary.MapRangeClamped` (`KismetMathLibrary.Abs` (`ChaosVehicleMovementComponent.GetForwardSpeedMPH` (`self.Vehicle Movement Component`))) 0.0 100.0 0.0 0.2)) 0.05 true false false false)
        (else
          ;[1 1 1] RightWheel On-Road Rumble
          (`self.PlayDynamicForceFeedback` (`KismetMathLibrary.MapRangeClamped` (/ (- _rightskid 500.0) 1000.0) 0.0 1.0 0.0 0.3) 0.05 false false false))))))

(fn `Find Skid Max`
  (returns (LeftSkid :type "Float (double-precision)") (RightSkid :type "Float (double-precision)") (LeftOffroad :type Boolean) (RightOffroad :type Boolean))
  (bind _vehicle_movement_component (`self.Vehicle Movement Component`))
  (bind (_bincontact _contactpoint _physmaterial _normalizedsuspensionlength _springforce _slipangle _bisslipping _slipmagnitude _bisskidding _skidmagnitude) (`ChaosWheeledVehicleMovementComponent.BreakWheelStatus` (`ChaosWheeledVehicleMovementComponent.GetWheelState` _vehicle_movement_component 0)))
  (bind (_bincontact_2 _contactpoint_2 _physmaterial_2 _normalizedsuspensionlength_2 _springforce_2 _slipangle_2 _bisslipping_2 _slipmagnitude_2 _bisskidding_2 _skidmagnitude_2) (`ChaosWheeledVehicleMovementComponent.BreakWheelStatus` (`ChaosWheeledVehicleMovementComponent.GetWheelState` _vehicle_movement_component 1)))
  (bind (_bincontact_3 _contactpoint_3 _physmaterial_3 _normalizedsuspensionlength_3 _springforce_3 _slipangle_3 _bisslipping_3 _slipmagnitude_3 _bisskidding_3 _skidmagnitude_3) (`ChaosWheeledVehicleMovementComponent.BreakWheelStatus` (`ChaosWheeledVehicleMovementComponent.GetWheelState` _vehicle_movement_component 2)))
  (bind (_bincontact_4 _contactpoint_4 _physmaterial_4 _normalizedsuspensionlength_4 _springforce_4 _slipangle_4 _bisslipping_4 _slipmagnitude_4 _bisskidding_4 _skidmagnitude_4) (`ChaosWheeledVehicleMovementComponent.BreakWheelStatus` (`ChaosWheeledVehicleMovementComponent.GetWheelState` _vehicle_movement_component 3)))
  (`KismetSystemLibrary.PrintString` (`KismetStringLibrary.Conv_DoubleToString` _slipmagnitude_4) true true (struct :`G` 0.66 :`B` 1.0 :`A` 1.0) 0.0)
  (return (`KismetMathLibrary.FMax` (* (`KismetMathLibrary.Conv_BoolToDouble` _bincontact) (`KismetMathLibrary.FMax` (`KismetMathLibrary.Abs` _slipmagnitude) (- (`KismetMathLibrary.Abs` _skidmagnitude) (`self.SkidAdjustment`)))) (* (`KismetMathLibrary.Conv_BoolToDouble` _bincontact_3) (`KismetMathLibrary.FMax` (`KismetMathLibrary.Abs` _slipmagnitude_3) (- (`KismetMathLibrary.Abs` _skidmagnitude_3) (`self.SkidAdjustment`))))) (`KismetMathLibrary.FMax` (* (`KismetMathLibrary.Conv_BoolToDouble` _bincontact_2) (`KismetMathLibrary.FMax` (`KismetMathLibrary.Abs` _slipmagnitude_2) (- (`KismetMathLibrary.Abs` _skidmagnitude_2) (`self.SkidAdjustment`)))) (* (`KismetMathLibrary.Conv_BoolToDouble` _bincontact_4) (`KismetMathLibrary.FMax` (`KismetMathLibrary.Abs` _slipmagnitude_4) (- (`KismetMathLibrary.Abs` _skidmagnitude_4) (`self.SkidAdjustment`))))) (or (and _bincontact_2 (!= _physmaterial_2 "/Game/PhysicsMaterials/Road.Road")) (and _bincontact_4 (!= _physmaterial_4 "/Game/PhysicsMaterials/Road.Road"))) (or (and _bincontact_3 (!= _physmaterial_3 "/Game/PhysicsMaterials/Road.Road")) (and _bincontact (!= _physmaterial "/Game/PhysicsMaterials/Road.Road")))))

(fn `Run Pause`
  (bind _returnvalue (`GameplayStatics.GetPlayerController` 0))
  (bind _returnvalue_2 (`KismetSystemLibrary.IsValid` (`self.PauseMenu`)))
  (`/Engine/EditorBlueprintResources/StandardMacros.IsValid` (`self.PauseMenu`)
    (:`Is Valid`
      (`CommonActivatableWidget.DeactivateWidget` (`self.PauseMenu`))
      (set `self.PauseMenu` null)
      (`WidgetBlueprintLibrary.SetInputMode_GameOnly` _returnvalue)
      (`AA_BaseUI.HidePauseOverlay` (`self.BaseUI`)))
    (:`Is Not Valid`
      (bind _returnvalue_3 (`AA_BaseUI.PushMenu` (`self.BaseUI`) "/Game/UI/UMG/Menus/UI_PauseMenu_BP.UI_PauseMenu_BP_C"))
      (set `self.PauseMenu` _returnvalue_3)
      (`WidgetBlueprintLibrary.SetInputMode_GameAndUIEx` _returnvalue null)
      (`AA_BaseUI.ShowPauseOverlay` (`self.BaseUI`))))
  (`GameplayStatics.SetGamePaused` _returnvalue_2)
  (set `PlayerController.bShowMouseCursor` _returnvalue_2 _returnvalue))

(fn `Toggle Map`
  (bind _returnvalue (subsystem `AA_MapCaptureSubsystem`))
  (bind _returnvalue_2 (subsystem `AA_MapCaptureSubsystem`))
  (bind _map_widget_class (`self.Map Widget Class`))
  (bind _current_map_widget (`self.Current Map Widget`))
  (`/Engine/EditorBlueprintResources/StandardMacros.IsValid` _current_map_widget
    (:`Is Valid`
      (`Widget.RemoveFromParent` _current_map_widget)
      (set `self.Current Map Widget` null)
      (`/Engine/EditorBlueprintResources/StandardMacros.IsValid` _returnvalue_2
        (:`Is Valid`
          (`AA_MapCaptureSubsystem.SetCaptureEnabled` _returnvalue_2 false))))
    (:`Is Not Valid`
      (if (`KismetSystemLibrary.IsValidSoftClassReference` _map_widget_class)
        (bind _returnvalue_3 (`KismetSystemLibrary.LoadClassAsset_Blocking` _map_widget_class))
        (bind _asuser_widget (castclass `UserWidget` _returnvalue_3))
        (`/Engine/EditorBlueprintResources/StandardMacros.IsValid` _returnvalue
          (:`Is Valid`
            (if (`AA_MapCaptureSubsystem.HasValidCaptureTarget` _returnvalue)
              (`AA_MapCaptureSubsystem.SetCaptureEnabled` _returnvalue true)
              (bind _returnvalue_4 (`|CreateWidget` _asuser_widget))
              (bind _output_get (set `self.Current Map Widget` _returnvalue_4))
              (`UserWidget.AddToViewport` _output_get 0))))))))

(fn `UserConstructionScript`)