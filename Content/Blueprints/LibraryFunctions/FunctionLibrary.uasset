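; Blueprint function library with one helper, ConvertFloatToTimeText, that turns a time in seconds into display text.
; Times over a minute read minutes:seconds.milliseconds with seconds zero-padded to two digits, while others omit the minutes.
; It splits stringified division and modulo results at the decimal point, truncating the fraction to at most three digits rather than rounding.
; The strict over-a-minute check makes exactly 60 seconds display without minutes.
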(fn ` `)

(fn `ConvertFloatToTimeText`
  (params (Time :type "Float (double-precision)"))
  (returns (TimeText :type Text))
  (bind _returnvalue (/ Time 60.0))
  (bind _returnvalue_2 (`KismetStringLibrary.ParseIntoArray` (`KismetStringLibrary.Conv_DoubleToString` (mod Time 60.0)) "."))
  (bind _output (`|GetArrayItem` _returnvalue_2))
  (bind _output_2 (`|GetArrayItem` (`KismetStringLibrary.ParseIntoArray` (`KismetStringLibrary.Conv_DoubleToString` _returnvalue) ".")))
  (bind _returnvalue_3 (`KismetStringLibrary.GetSubstring` (`|GetArrayItem` _returnvalue_2 1) 0 3))
  ;[1 1 1] If Over A Minute
  (if (> _returnvalue 1.0)
    ;[1 1 1] If Seconds has only 1 digit
    (if (== (`KismetStringLibrary.Len` _output) 1)
      ;[1 1 1] When Seconds are Under 10, and Minute >= 1, Prefix seconds with a 0
      (return (`KismetTextLibrary.Conv_StringToText` (`KismetStringLibrary.Concat_StrStr` _output_2 ":" "0" _output "." _returnvalue_3)))
      (else
        ;[1 1 1] Set Time Normally
        (return (`KismetTextLibrary.Conv_StringToText` (`KismetStringLibrary.Concat_StrStr` _output_2 ":" _output "." _returnvalue_3)))))
    (else
      ;[1 1 1] Set Time when Under a minute
      (return (`KismetTextLibrary.Conv_StringToText` (`KismetStringLibrary.Concat_StrStr` _output "." _returnvalue_3))))))