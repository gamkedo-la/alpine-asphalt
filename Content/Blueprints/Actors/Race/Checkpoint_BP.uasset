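; Race checkpoint actor that marks itself with a light and a flare on each of its left and right sides.
; On BeginPlay it shifts each pair along local Y by the LeftLocation and RightLocation offsets, hides the lights, deactivates the flares and zeroes their world rotation.
; A SetActive event toggles both lights and flares together.
; It contains no overlap or progress logic of its own.
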(event `self.ReceiveBeginPlay`
  (bind _leftlocation (`self.LeftLocation`))
  (bind _leftflare (`self.LeftFlare`))
  (bind _rightflare (`self.RightFlare`))
  (bind _rightlocation (`self.RightLocation`))
  (`SceneComponent.K2_AddLocalOffset` (`self.LeftLight`) (`KismetMathLibrary.MakeVector` 0.0 _leftlocation) false false)
  (`SceneComponent.K2_AddLocalOffset` (`self.RightLight`) (`KismetMathLibrary.MakeVector` 0.0 _rightlocation) false false)
  (`SceneComponent.K2_AddLocalOffset` (`self.LeftFlare`) (`KismetMathLibrary.MakeVector` 0.0 _leftlocation) false false)
  (`SceneComponent.K2_AddLocalOffset` (`self.RightFlare`) (`KismetMathLibrary.MakeVector` 0.0 _rightlocation) false false)
  (`SceneComponent.SetVisibility` (`self.LeftLight`) false false)
  (`SceneComponent.SetVisibility` (`self.RightLight`) false false)
  (`ActorComponent.SetActive` _leftflare false false)
  (`ActorComponent.SetActive` _rightflare false false)
  (`SceneComponent.K2_SetWorldRotation` :`self` _leftflare)
  (`SceneComponent.K2_SetWorldRotation` :`self` _rightflare))

(event `self.SetActive`
  (params (IsActive :type Boolean))
  (`SceneComponent.SetVisibility` (`self.LeftLight`) IsActive false)
  (`SceneComponent.SetVisibility` (`self.RightLight`) IsActive false)
  (`ActorComponent.SetActive` (`self.LeftFlare`) IsActive false)
  (`ActorComponent.SetActive` (`self.RightFlare`) IsActive false))

(fn `UserConstructionScript`)