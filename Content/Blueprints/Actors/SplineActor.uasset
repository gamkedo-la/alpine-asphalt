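; SplineActor populates its spline with copies of a configurable actor class when play begins.
; SpawnActors steps along the spline at a fixed spacing, spawning each actor with the spline's world location and rotation at that distance.
; The SpawnedActors array length serves as the step counter and is cleared afterwards, so no references to the spawned actors are retained there.
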(event `self.ReceiveBeginPlay`
  (`self.SpawnActors`))

(fn `SpawnActors`
  (bind _spline (`self.Spline`))
  (bind _returnvalue (* (`KismetArrayLibrary.Array_Length` (`self.Spawned Actors`)) (`self.DistanceBetweenActors`)))
  (while (< (* (`KismetArrayLibrary.Array_Length` (`self.Spawned Actors`)) (`self.DistanceBetweenActors`)) (`SplineComponent.GetSplineLength` (`self.Spline`)))
    (bind _returnvalue_2 (`|SpawnActorFromClass` (`self.ActorToSpawn`) (`KismetMathLibrary.MakeTransform` (`SplineComponent.GetLocationAtDistanceAlongSpline` _spline _returnvalue "World") (`SplineComponent.GetRotationAtDistanceAlongSpline` _spline _returnvalue "World")) "Undefined" "MultiplyWithRoot" self null))
    (`KismetArrayLibrary.Array_Add` (`self.Spawned Actors`) _returnvalue_2))
  (`KismetArrayLibrary.Array_Clear` (`self.Spawned Actors`)))

(fn `UserConstructionScript`)