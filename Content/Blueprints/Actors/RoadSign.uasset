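; RoadSign is an actor that returns its physics-driven mesh to its starting pose after being knocked by a hit.
; BeginPlay caches the mesh's world transform.
; The first component hit passes a DoOnce, waits a configurable delay, restores location and rotation, puts the rigid body to sleep, then resets the gate for the next hit.
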(event `self.ReceiveBeginPlay`
  (set `self.Original Transform` (`SceneComponent.K2_GetComponentToWorld` (`self.StaticMesh`))))

(event `self.StaticMesh.OnComponentHit`
  (params (HitComponent :type "PrimitiveComponent Object Reference") (OtherActor :type "Actor Object Reference") (OtherComp :type "PrimitiveComponent Object Reference") (NormalImpulse :type "Vector Structure") (Hit :type "HitResult Structure (by ref)"))
  (bind (_original_transform_location _original_transform_rotation) (`KismetMathLibrary.BreakTransform` (`self.Original Transform`)))
  (`/Engine/EditorBlueprintResources/StandardMacros.DoOnce` false :!label _label
    (:`Completed`
      (`KismetSystemLibrary.Delay` (`self.Time`))
      (`SceneComponent.K2_SetWorldLocationAndRotation` (`self.StaticMesh`) _original_transform_location _original_transform_rotation false false)
      (`PrimitiveComponent.PutRigidBodyToSleep` (`self.StaticMesh`) "None")
      (goto _label :!via `Reset`))))

(fn `UserConstructionScript`)