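; Player controller for a drivable vehicle, handling the driving HUD, controller rumble and pause menu.
; BeginPlay creates the HUD and caches the vehicle's movement component, which Tick reads to update speed and gear.
; While skidding, Tick plays small-motor force feedback scaled by FindSkidMax, which reads only wheel 0 despite its four-way max.
; The pause input toggles the menu widget, game pause, input mode and mouse cursor.
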(event `EnhancedInput|/Game/Input/Actions/IA_Pause`
  (params (ActionValue :type Boolean) (ElapsedSeconds :type "Float (double-precision)") (TriggeredSeconds :type "Float (double-precision)") (InputAction :type "InputAction Object Reference" :default "/Game/Input/Actions/IA_Pause.IA_Pause"))
  (:`Completed`
    (`self.Run Pause`)))

(event `self.ReceiveBeginPlay`
  (bind _returnvalue (`|CreateWidget` "/Game/Blueprints/VehicleUI.VehicleUI_C" self))
  (bind _output_get (set `self.VehicleHud` _returnvalue))
  (`UserWidget.AddToViewport` _output_get 0)
  (bind _asvehicle_pawn_bp (cast `/Game/Blueprints/VehiclePawn_BP` (`self.K2_GetPawn`)))
  (set `self.Vehicle Movement Component` (`AA_WheeledVehiclePawn.VehicleMovementComponent` _asvehicle_pawn_bp)))

(event `self.ReceiveTick`
  (params (DeltaSeconds :type "Float (single-precision)"))
  (bind _vehicle_movement_component (`self.Vehicle Movement Component`))
  (`/Game/Blueprints/VehicleUI.UpdateSpeed` (`self.VehicleHud`) (`ChaosVehicleMovementComponent.GetForwardSpeed` _vehicle_movement_component))
  (`/Game/Blueprints/VehicleUI.UpdateGear` (`self.VehicleHud`) (`ChaosVehicleMovementComponent.GetCurrentGear` _vehicle_movement_component))
  (bind (_returnvalue _bisskidding) (`self.Find Skid Max`))
  (if _bisskidding
    (`self.PlayDynamicForceFeedback` _returnvalue 0.1 false true false)))

(fn `Find Skid Max`
  (returns (ReturnValue :type "Float (double-precision)") (bIsSkidding :type Boolean))
  (bind _vehicle_movement_component (`self.Vehicle Movement Component`))
  (bind (_bincontact _contactpoint _physmaterial _normalizedsuspensionlength _springforce _slipangle _bisslipping _slipmagnitude _bisskidding _skidmagnitude) (`ChaosWheeledVehicleMovementComponent.BreakWheelStatus` (`ChaosWheeledVehicleMovementComponent.GetWheelState` _vehicle_movement_component 0)))
  (return (/ (`KismetMathLibrary.Abs` (`KismetMathLibrary.FMax` (`KismetMathLibrary.FMax` (`KismetMathLibrary.FMax` _skidmagnitude (`.SkidMagnitude` (`ChaosWheeledVehicleMovementComponent.BreakWheelStatus` (`ChaosWheeledVehicleMovementComponent.GetWheelState` _vehicle_movement_component 0)))) (`.SkidMagnitude` (`ChaosWheeledVehicleMovementComponent.BreakWheelStatus` (`ChaosWheeledVehicleMovementComponent.GetWheelState` _vehicle_movement_component 0)))) (`.SkidMagnitude` (`ChaosWheeledVehicleMovementComponent.BreakWheelStatus` (`ChaosWheeledVehicleMovementComponent.GetWheelState` _vehicle_movement_component 0))))) 10000.0) _bisskidding))

(fn `Run Pause`
  (bind _returnvalue (`GameplayStatics.GetPlayerController` 0))
  (bind _pausemenu (`self.PauseMenu`))
  (bind _returnvalue_2 (`KismetSystemLibrary.IsValid` (`self.PauseMenu`)))
  (`/Engine/EditorBlueprintResources/StandardMacros.IsValid` _pausemenu
    (:`Is Valid`
      (`Widget.RemoveFromParent` _pausemenu)
      (set `self.PauseMenu` null)
      (`WidgetBlueprintLibrary.SetInputMode_GameOnly` _returnvalue))
    (:`Is Not Valid`
      (bind _returnvalue_3 (`|CreateWidget` "/Game/UMG/UMG_PauseMenu.UMG_PauseMenu_C" self))
      (bind _output_get (set `self.PauseMenu` _returnvalue_3))
      (`UserWidget.AddToViewport` _output_get 0)
      (`WidgetBlueprintLibrary.SetInputMode_GameAndUIEx` _returnvalue null)))
  (`GameplayStatics.SetGamePaused` _returnvalue_2)
  (set `PlayerController.bShowMouseCursor` _returnvalue_2 _returnvalue))

(fn `UserConstructionScript`)