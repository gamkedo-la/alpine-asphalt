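; Race actor that starts a vehicle race when the E key is pressed.
; It hides every entry in its Checkpoints array at BeginPlay.
; On E it loops through them to reveal each one, calling Countdown on the vehicle player controller's HUD and hiding itself in game.
; The countdown and hide calls sit inside the loop body, so they repeat for each checkpoint.
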(event `self.ReceiveBeginPlay`
  (for _array_element (`self.Checkpoints`)
    (`/Game/Blueprints/Checkpoint.SetVisibility` _array_element false)))

(event `Key|E`
  (params (Key :type "Key Structure"))
  (:`Pressed`
    (for _array_element (`self.Checkpoints`)
      (`/Game/Blueprints/Checkpoint.SetVisibility` _array_element true)
      (bind _asvehicle_player_controller_bp (cast `/Game/Blueprints/VehiclePlayerController_BP` (`GameplayStatics.GetPlayerController` 0)))
      (`/Game/Blueprints/VehicleUI.Countdown` (`/Game/Blueprints/VehiclePlayerController_BP.VehicleHud` _asvehicle_player_controller_bp))
      (`self.SetActorHiddenInGame` true))))

(fn `UserConstructionScript`)