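; BP_Minimap is an actor that puts the minimap widget on screen and supplies it with player tracking data.
; On BeginPlay it creates WBP_Minimap and adds it to the viewport.
; Each tick it writes the first player controller's location and yaw into the MP_Minimap material parameter collection.
; Negative yaw is wrapped and normalized to the 0–1 range the material requires.
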(event `self.ReceiveBeginPlay`
  (bind _returnvalue (`|CreateWidget` "/Game/UI/Map/WBP_Minimap.WBP_Minimap_C"))
  (`UserWidget.AddToViewport` _returnvalue 0))

(event `self.ReceiveTick`
  (params (DeltaSeconds :type "Float (single-precision)"))
  (bind _returnvalue (`GameplayStatics.GetPlayerController` 0))
  (bind (_returnvalue_roll _returnvalue_pitch _returnvalue_yaw) (`KismetMathLibrary.BreakRotator` (`self.K2_GetActorRotation` _returnvalue)))
  (`/Engine/EditorBlueprintResources/StandardMacros.IsValid` _returnvalue
    (:`Is Valid`
      (`KismetMaterialLibrary.SetVectorParameterValue` "/Game/Artwork/Materials/Map/MP_Minimap.MP_Minimap" "PlayerLocation" (`KismetMathLibrary.Conv_VectorToLinearColor` (`self.K2_GetActorLocation` _returnvalue)))
      (`KismetMaterialLibrary.SetScalarParameterValue` "/Game/Artwork/Materials/Map/MP_Minimap.MP_Minimap" "PlayerYaw" (/ (`KismetMathLibrary.SelectFloat` (+ _returnvalue_yaw 360.0) _returnvalue_yaw (< _returnvalue_yaw 0.0)) 360.0)))))

(fn `UserConstructionScript`)